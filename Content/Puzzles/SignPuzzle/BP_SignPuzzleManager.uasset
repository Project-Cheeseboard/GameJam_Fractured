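; Manager for the sign puzzle that opens a door when buttons are entered in the correct order.
; CheckButtons appends and prints each button ID, then CheckCombination compares the entered code to the correct one once their lengths match.
; A match sets PuzzleComplete and plays a timeline that raises the Cube.
; A mismatch clears the entry and calls PuzzleFail on the referenced sign puzzle.
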(event `OpenDoor`
  (if (`self.bPuzzleComplete`)
    (bind (_direction _newtrack_0) (`Timeline|OpeningDoor`)
      (:`Update`
        (`SceneComponent.K2_SetRelativeLocation` (`self.Cube`) (`KismetMathLibrary.MakeVector` 0.0 0.0 (`KismetMathLibrary.Lerp` 0.0 125.0 _newtrack_0)) false false)))))

(fn `CheckButtons`
  (params (ButtonID :type Integer))
  (`KismetArrayLibrary.Array_Add` (`self.EnteredCode`) ButtonID)
  (`KismetSystemLibrary.PrintString` (`KismetStringLibrary.Conv_IntToString` ButtonID))
  (`self.CheckCombination`))

(fn `CheckCombination`
  (set `self.bCombinationValid` true)
  (if (== (`KismetArrayLibrary.Array_Length` (`self.EnteredCode`)) (`KismetArrayLibrary.Array_Length` (`self.CorrectCode`)))
    (for (_array_element _array_index) (`self.CorrectCode`)
      (if (not (== _array_element (`|GetArrayItem` (`self.EnteredCode`) _array_index)))
        (set `self.bCombinationValid` false)))
    (if (`self.bCombinationValid`)
      (set `self.bPuzzleComplete` true)
      (`self.OpenDoor`)
      (else
        (`KismetArrayLibrary.Array_Clear` (`self.EnteredCode`))
        (`/Game/Puzzles/SignPuzzle/BP_SignPuzzle.PuzzleFail` (`self.SignPuzzleRef`))))))

(fn `UserConstructionScript`)