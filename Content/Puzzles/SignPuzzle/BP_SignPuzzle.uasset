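; Nine-button keypad actor for the sign puzzle, interactable until its puzzle manager reports the puzzle complete.
; At BeginPlay each button gets a dynamic keypad material, stored in an array.
; Interacting converts ButtonName to a number, lights that button through the IsOn parameter and passes the number to the manager's CheckButtons.
; PuzzleFail switches every button off after a short delay.
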(event `self.ReceiveBeginPlay`
  (for _array_element (`|MakeArray` (`self.Button1`) (`self.Button2`) (`self.Button3`) (`self.Button4`) (`self.Button5`) (`self.Button6`) (`self.Button7`) (`self.Button8`) (`self.Button9`))
    (bind _returnvalue (`PrimitiveComponent.CreateDynamicMaterialInstance` _array_element 0 "/Game/Puzzles/PiggyPuzzle/M_KeyPadButton.M_KeyPadButton" "None"))
    (`KismetArrayLibrary.Array_Add` (`self.ButtonMaterials`) _returnvalue)))

(event `self.Interact`
  (params (Player :type "/Game/FPMovement/Player/Blueprints/BP_Player Object Reference"))
  (bind _buttonmaterials (`self.ButtonMaterials`))
  (bind _returnvalue (`KismetStringLibrary.Conv_StringToInt` (`KismetStringLibrary.Conv_NameToString` (`self.ButtonName`))))
  (bind _returnvalue_2 (- _returnvalue 1))
  (if (`KismetArrayLibrary.Array_IsValidIndex` _buttonmaterials _returnvalue_2)
    (`MaterialInstanceDynamic.SetScalarParameterValue` (`|GetArrayItem` _buttonmaterials _returnvalue_2) "IsOn" 1.0)
    (`/Game/Puzzles/SignPuzzle/BP_SignPuzzleManager.CheckButtons` (`self.PuzzleManagerRef`) _returnvalue)
    (`KismetSystemLibrary.PrintString` (`KismetStringLibrary.Conv_IntToString` _returnvalue_2))))

(event `PuzzleFail`
  (`KismetSystemLibrary.Delay` 0.2)
  (for _array_element (`self.ButtonMaterials`)
    (`MaterialInstanceDynamic.SetScalarParameterValue` _array_element "IsOn" 0.0)))

(fn `Can_Interact?`
  (returns (`CanInteract?` :type Boolean))
  (return (not (`/Game/Puzzles/SignPuzzle/BP_SignPuzzleManager.bPuzzleComplete` (`self.PuzzleManagerRef`)))))

(fn `Interact_Prompt`
  (returns (`ShowPrompt?` :type Boolean) (Name :type Name))
  (return (`self.bShowPrompt`) (`self.ButtonName`)))

(fn `UserConstructionScript`)