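; Interactable toggle button for the bridge puzzle that holds its own on/off state and ID.
; Interact flips the state, sets a matching parameter on the button's dynamic material and plays a timeline forward or in reverse to slide the button mesh.
; CanInteract and InteractPrompt expose availability and prompt details.
; The timeline update also prints the ID and state, and nothing here drives the bridge directly.
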(event `self.ReceiveBeginPlay`
  (bind _returnvalue (`PrimitiveComponent.CreateDynamicMaterialInstance` (`self.Button`) 0 "/Game/Puzzles/BridgePuzzle/M_BridgeButton.M_BridgeButton" "None"))
  (set `self.ButtonMaterial` _returnvalue))

(event `/Game/FPMovement/Player/Blueprints/Interface/BP_Interact.Interact`
  (params (Player :type "/Game/FPMovement/Player/Blueprints/BP_Player Object Reference"))
  (set `self.bIsOn` (not (`self.bIsOn`)))
  (`MaterialInstanceDynamic.SetScalarParameterValue` (`self.ButtonMaterial`) "IsOn" (`KismetMathLibrary.SelectFloat` 1.0 0.0 (`self.bIsOn`)))
  (if (`self.bIsOn`)
    (bind (_direction _buttonpress) (`Timeline|ButtonPress` :!via `PlayFromStart` :!label _label)
      (:`Update`
        (`SceneComponent.K2_SetRelativeLocation` (`self.Button`) (`KismetMathLibrary.MakeVector` 0.0 (`KismetMathLibrary.Lerp` 45.0 25.0 _buttonpress)) false false)
        (`KismetSystemLibrary.PrintString` (`KismetStringLibrary.Concat_StrStr` (`KismetStringLibrary.Conv_IntToString` (`self.ButtonID`)) (`KismetStringLibrary.Conv_BoolToString` (`self.bIsOn`))))))
    (else
      (goto _label :!via `ReverseFromEnd`))))

(fn `Can_Interact?`
  (returns (`CanInteract?` :type Boolean))
  (return (`self.bCanInteract`)))

(fn `Interact_Prompt`
  (returns (`ShowPrompt?` :type Boolean) (Name :type Name))
  (return (`self.bShowPrompt`) (`self.ButtonName`)))

(fn `UserConstructionScript`)