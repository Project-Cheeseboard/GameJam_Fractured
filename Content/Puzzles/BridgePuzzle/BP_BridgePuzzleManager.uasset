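; BP_BridgePuzzleManager runs a button-combination puzzle that raises a bridge when solved.
; CheckButtons adds or removes a button ID in ActiveButtons as it toggles, then calls CheckCombination.
; CheckCombination compares ActiveButtons with CorrectButtons by count and membership, so press order is irrelevant.
; A match sets PuzzleComplete, which ignores further input, prints a message and calls RaiseBridge on BridgeRef.
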(fn `CheckButtons`
  (params (ButtonID :type Integer) (IsOn :type Boolean))
  (if (`self.bPuzzleComplete`)
    _
    (elif IsOn
      (`KismetArrayLibrary.Array_AddUnique` (`self.ActiveButtons`) ButtonID)
      (`self.CheckCombination`)
      (else
        (`KismetArrayLibrary.Array_RemoveItem` (`self.ActiveButtons`) ButtonID)
        (`self.CheckCombination`)))))

(fn `CheckCombination`
  (set `self.bCombinationValid` true)
  (if (== (`KismetArrayLibrary.Array_Length` (`self.ActiveButtons`)) (`KismetArrayLibrary.Array_Length` (`self.CorrectButtons`)))
    (for _array_element (`self.CorrectButtons`)
      (if (not (`KismetArrayLibrary.Array_Contains` (`self.ActiveButtons`) _array_element))
        (set `self.bCombinationValid` false)))
    (if (`self.bCombinationValid`)
      (set `self.bPuzzleComplete` true)
      (`KismetSystemLibrary.PrintString` "bridge puzzle complete")
      (`/Game/Puzzles/BridgePuzzle/BP_Bridge.RaiseBridge` (`self.BridgeRef`)))))

(fn `UserConstructionScript`)