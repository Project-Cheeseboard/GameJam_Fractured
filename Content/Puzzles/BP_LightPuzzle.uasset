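; BP_LightPuzzle is a puzzle light that turns its spotlight green when the player lingers in its trigger.
; Overlap events on LightTrigger track player presence in a flag, which is rechecked after a short Delay before the colour changes.
; Activation prints the light's ID for debugging.
; Leaving clears the flag but does not revert the colour.
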(event `self.Light Trigger.OnComponentBeginOverlap`
  (params (OverlappedComponent :type "PrimitiveComponent Object Reference") (OtherActor :type "Actor Object Reference") (OtherComp :type "PrimitiveComponent Object Reference") (OtherBodyIndex :type Integer) (bFromSweep :type Boolean) (SweepResult :type "HitResult Structure (by ref)"))
  (cast `/Game/FPMovement/Player/Blueprints/BP_Player` OtherActor
    (:`then`
      (set `self.bPlayerInTrigger` true)
      (`KismetSystemLibrary.Delay` 3.0)
      (if (`self.bPlayerInTrigger`)
        (`LightComponent.SetLightColor` (`self.SpotLight`) (struct :`G` 1.0 :`A` 1.0) true)
        (`KismetSystemLibrary.PrintString` (`KismetStringLibrary.Concat_StrStr` "Light Active: " (`KismetStringLibrary.Conv_IntToString` (`self.LightID`))))))
    (:`CastFailed`
      (`KismetSystemLibrary.PrintString` "Fail at light trigger player cast"))))

(event `self.Light Trigger.OnComponentEndOverlap`
  (params (OverlappedComponent :type "PrimitiveComponent Object Reference") (OtherActor :type "Actor Object Reference") (OtherComp :type "PrimitiveComponent Object Reference") (OtherBodyIndex :type Integer))
  (cast `/Game/FPMovement/Player/Blueprints/BP_Player` OtherActor
    (:`then`
      (set `self.bPlayerInTrigger` false)
      (`KismetSystemLibrary.PrintString` "Player has left"))
    (:`CastFailed`
      (`KismetSystemLibrary.PrintString` "fail at light trigger player cast"))))

(fn `UserConstructionScript`)