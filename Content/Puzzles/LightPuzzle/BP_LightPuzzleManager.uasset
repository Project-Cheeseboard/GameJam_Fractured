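; BP_LightPuzzleManager runs a sequence puzzle in which lights must be triggered in the correct order.
; CheckLight compares each light ID to the next step of the correct sequence; a wrong one resets progress and calls PuzzleFail on every puzzle light.
; Completing the sequence locks the puzzle, spawns a BP_BaseKey pickup at the key spawn point and reveals a highlight component.
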(event `PuzzleSuccess`
  (`|SpawnActorFromClass` "/Game/FPMovement/Blueprints/Doors/BP_BaseKey.BP_BaseKey_C" (`SceneComponent.K2_GetComponentToWorld` (`self.KeySpawnPoint`)) "AlwaysSpawn" "MultiplyWithRoot" null 1 true "Key" "has been picked up" (struct) null)
  (`SceneComponent.SetVisibility` (`self.Highlight`) true false))

(fn `CheckLight`
  (params (LightID :type Integer))
  (if (`self.bPuzzleComplete`)
    _
    (elif (== LightID (`|GetArrayItem` (`self.CorrectSequence`) (`self.CurrentStep`)))
      (set `self.CurrentStep` (+ (`self.CurrentStep`) 1))
      (if (== (`KismetArrayLibrary.Array_Length` (`self.CorrectSequence`)) (`self.CurrentStep`))
        (set `self.bPuzzleComplete` true)
        (`self.PuzzleSuccess`)
        (`KismetSystemLibrary.PrintString` "Puzzle Complete"))
      (else
        (set `self.CurrentStep` 0)
        (for _array_element (`self.PuzzleLights`)
          (`/Game/Puzzles/LightPuzzle/BP_LightPuzzle.PuzzleFail` _array_element))
        (`KismetSystemLibrary.PrintString` "Wrong Light - Puzzle Reset")))))

(fn `UserConstructionScript`)