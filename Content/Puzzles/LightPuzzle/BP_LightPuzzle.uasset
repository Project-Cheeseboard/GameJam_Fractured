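; A puzzle light that the player activates by standing in its trigger, one element of a light puzzle run by a referenced puzzle manager.
; If the player is still inside after a short delay and the puzzle is incomplete, the spotlight turns green and reports its LightID to the manager's CheckLight.
; PuzzleFail flashes the light dark red, then restores its warm color and makes it inactive again.
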(event `self.Light Trigger.OnComponentBeginOverlap`
  (params (OverlappedComponent :type "PrimitiveComponent Object Reference") (OtherActor :type "Actor Object Reference") (OtherComp :type "PrimitiveComponent Object Reference") (OtherBodyIndex :type Integer) (bFromSweep :type Boolean) (SweepResult :type "HitResult Structure (by ref)"))
  (cast `/Game/FPMovement/Player/Blueprints/BP_Player` OtherActor
    (:`then`
      (set `self.bPlayerInTrigger` true)
      (if (`/Game/Puzzles/LightPuzzle/BP_LightPuzzleManager.bPuzzleComplete` (`self.PuzzleManagerRef`))
        (`KismetSystemLibrary.PrintString` "Puzzle already complete")
        (else
          (`KismetSystemLibrary.Delay` 3.0)
          (if (`self.bPlayerInTrigger`)
            (if (not (`self.bActiveLight`))
              (`LightComponent.SetLightColor` (`self.SpotLight`) (struct :`G` 1.0 :`A` 1.0) true)
              (set `self.bActiveLight` true)
              (`KismetSystemLibrary.PrintString` (`KismetStringLibrary.Concat_StrStr` "Light Active: " (`KismetStringLibrary.Conv_IntToString` (`self.LightID`))))
              (`/Game/Puzzles/LightPuzzle/BP_LightPuzzleManager.CheckLight` (`self.PuzzleManagerRef`) (`self.LightID`)))))))
    (:`CastFailed`
      (`KismetSystemLibrary.PrintString` "Fail at light trigger player cast"))))

(event `self.Light Trigger.OnComponentEndOverlap`
  (params (OverlappedComponent :type "PrimitiveComponent Object Reference") (OtherActor :type "Actor Object Reference") (OtherComp :type "PrimitiveComponent Object Reference") (OtherBodyIndex :type Integer))
  (cast `/Game/FPMovement/Player/Blueprints/BP_Player` OtherActor
    (:`then`
      (`KismetSystemLibrary.PrintString` "Player has left")
      (set `self.bPlayerInTrigger` false))
    (:`CastFailed`
      (`KismetSystemLibrary.PrintString` "fail at light trigger player cast"))))

(event `PuzzleFail`
  (`LightComponent.SetLightColor` (`self.SpotLight`) (struct :`R` 0.416001 :`A` 1.0) true)
  (`KismetSystemLibrary.Delay` 1.0)
  (`LightComponent.SetLightColor` (`self.SpotLight`) (struct :`R` 0.723055 :`G` 0.637597 :`B` 0.327778 :`A` 1.0) true)
  (set `self.bActiveLight` false))

(fn `UserConstructionScript`)