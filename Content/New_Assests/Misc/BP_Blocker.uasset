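; BP_Blocker is a trigger actor that seals a route behind the player once they have passed through it.
; Overlaps with detection points A and B set flags, and leaving B with both set enables the Wall's collision and visibility.
; It also spawns a locked BP_BaseDoor at the Arrow's transform, then clears both flags, with debug prints tracing each step.
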(event `self.DetectionPointA.OnComponentBeginOverlap`
  (params (OverlappedComponent :type "PrimitiveComponent Object Reference") (OtherActor :type "Actor Object Reference") (OtherComp :type "PrimitiveComponent Object Reference") (OtherBodyIndex :type Integer) (bFromSweep :type Boolean) (SweepResult :type "HitResult Structure (by ref)"))
  (cast `/Game/FPMovement/Player/Blueprints/BP_Player` OtherActor
    (:`then`
      (`KismetSystemLibrary.PrintString` "Player has past point a")
      (set `self.bDetectionPointA` true))
    (:`CastFailed`
      (`KismetSystemLibrary.PrintString` "Cast failed at BP_Blocker Point A"))))

(event `self.DetectionPointB.OnComponentBeginOverlap`
  (params (OverlappedComponent :type "PrimitiveComponent Object Reference") (OtherActor :type "Actor Object Reference") (OtherComp :type "PrimitiveComponent Object Reference") (OtherBodyIndex :type Integer) (bFromSweep :type Boolean) (SweepResult :type "HitResult Structure (by ref)"))
  (cast `/Game/FPMovement/Player/Blueprints/BP_Player` OtherActor
    (:`then`
      (`KismetSystemLibrary.PrintString` "Player has past point b")
      (set `self.bDetectionPointB` true))
    (:`CastFailed`
      (`KismetSystemLibrary.PrintString` "Cast failed at BP_Blocker Point B"))))

(event `self.DetectionPointB.OnComponentEndOverlap`
  (params (OverlappedComponent :type "PrimitiveComponent Object Reference") (OtherActor :type "Actor Object Reference") (OtherComp :type "PrimitiveComponent Object Reference") (OtherBodyIndex :type Integer))
  (bind _wall (`self.Wall`))
  (cast `/Game/FPMovement/Player/Blueprints/BP_Player` OtherActor
    (:`then`
      (if (and (`self.bDetectionPointA`) (`self.bDetectionPointB`))
        (`PrimitiveComponent.SetCollisionEnabled` _wall "QueryAndPhysics")
        (`SceneComponent.SetVisibility` _wall true false)
        (`|SpawnActorFromClass` "/Game/FPMovement/Blueprints/Doors/BP_BaseDoor.BP_BaseDoor_C" (`SceneComponent.K2_GetComponentToWorld` (`self.Arrow`)) "Undefined" "MultiplyWithRoot" null true 999 100.0 30.0 "/Game/FPMovement/Assets/Audio/Abilitys/Door/SW_Key_Insertion.SW_Key_Insertion" "/Game/FPMovement/Assets/Audio/Abilitys/Door/SW_Open_Door.SW_Open_Door" "/Game/FPMovement/Assets/Audio/Abilitys/Door/SW_Close_Door.SW_Close_Door" "/Game/FPMovement/Assets/Audio/Abilitys/Door/SW_TryOpen_Door.SW_TryOpen_Door" true "Close Door" "Open Door" "as been unlocked" "Door" (struct) null)
        (`KismetSystemLibrary.PrintString` "Route Blocked")
        (set `self.bDetectionPointA` false)
        (set `self.bDetectionPointB` false)))
    (:`CastFailed`
      (`KismetSystemLibrary.PrintString` "Cast failed at BP_Blocker End Overlap"))))

(fn `UserConstructionScript`)